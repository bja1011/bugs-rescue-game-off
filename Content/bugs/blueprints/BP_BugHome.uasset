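; BP_BugHome is a bug's home actor that displays the display name of its owner bug as floating text.
; On BeginPlay it adds a text render component and fills it with the OwnerBugRef name.
; Each Tick it rotates the label using a look-at between the forward vectors of the BP_Player mesh and the home mesh, rather than their world locations.
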(event EventBeginPlay
  (bind _returnvalue (AddComponent|AddTextRenderComponent false))
  (Rendering|Components|TextRender|SetText _returnvalue (Utilities|Text|ToText(String) (Utilities|GetDisplayName (Variables|Default|GetOwnerBugRef)))))

(event Collision|EventActorBeginOverlap
  (params (OtherActor :type Actor%20Object%20Reference)))

(event EventTick
  (params (DeltaSeconds :type Float%20%28single-precision%29))
  (Utilities|IsValid (stale EventBeginPlay _returnvalue)
    (:Is%20Valid
      (bind _asbp_player (Utilities|Casting|CastToBP_Player (Pawn|GetControlledPawn (Game|GetPlayerController 0))))
      (Transformation|SetWorldRotation (stale EventBeginPlay _returnvalue) (Math|Rotator|FindLookatRotation (Math|Rotator|GetRotationXVector (Transformation|GetWorldRotation (Variables|/Game/player/blueprints/BP_Player.BP_Player_C|GetPlayerMesh _asbp_player))) (Math|Rotator|GetRotationXVector (Transformation|GetWorldRotation (Variables|Default|GetBugHomeMesh)))) false false))))

(fn ConstructionScript)