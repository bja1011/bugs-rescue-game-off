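; Game mode that provides the logic for a bug calling for help.
; CallForHelp stores a valid bug reference, unhides that actor and shows a focusable BP_NeedHelpUI widget built from the bug's Info.
; FindBugToHelp simply returns the first BP_bug actor in the world, with no further selection.
; BeginPlay and Tick are disabled stubs, so nothing in this graph triggers either function.
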(event EventBeginPlay)

(event EventTick
  (params (DeltaSeconds :type Float%20%28single-precision%29)))

(fn ConstructionScript)

(fn CallforHelp
  (params (BugToHelpRef :type BP%20Bug%20Object%20Reference%20%28by%20ref%29))
  (if (Utilities|IsValid BugToHelpRef)
    (bind _output_get (Variables|Default|SetBugToHelpRef BugToHelpRef))
    (Rendering|SetActorHiddenInGame _output_get false)
    (bind _returnvalue (UserInterface|CreateWidget "/Game/UI/BP_NeedHelpUI.BP_NeedHelpUI_C" 0 (Variables|/Game/bugs/blueprints/BP_bug.BP_bug_C|GetInfo _output_get)))
    (UserInterface|Viewport|AddtoViewport _returnvalue 1)
    (Variables|/Script/UMG.UserWidget|SetbIsFocusable _returnvalue true)))

(fn FindBugtoHelp
  (bind _outactors (Actor|GetAllActorsOfClass "/Game/bugs/blueprints/BP_bug.BP_bug_C"))
  (return (Utilities|Array|Get(acopy) _outactors)))