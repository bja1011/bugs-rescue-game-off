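; BP_RescueHome is an actor marking a home zone where the player triggers bug rescue requests.
; It caches BP_GameMode on BeginPlay.
; Every Tick, while the game mode has no valid bug to help, each player overlapping its sphere makes the game mode find a bug and call for help.
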(event EventBeginPlay
  (bind _asbp_game_mode (Utilities|Casting|CastToBP_GameMode (Game|GetGameMode)))
  (Variables|Default|SetGameMode _asbp_game_mode))

(event EventTick
  (params (DeltaSeconds :type Float%20%28single-precision%29))
  (bind _gamemode (Variables|Default|GetGameMode))
  (if (not (Utilities|IsValid (Variables|/Game/game/BP_GameMode.BP_GameMode_C|GetBugToHelpRef (Variables|Default|GetGameMode))))
    (for _array_element (Collision|GetOverlappingActors (Variables|Default|GetSphere) "/Game/player/blueprints/BP_Player.BP_Player_C" :!class /Script/Engine.PrimitiveComponent)
      (if true
        (bind _foundbug (Default|FindBugtoHelp _gamemode))
        (Default|CallforHelp _gamemode _foundbug)))))

(fn ConstructionScript)