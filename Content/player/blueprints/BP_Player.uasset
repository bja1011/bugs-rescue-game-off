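; Player pawn for a physics-driven flyer that rescues bugs, carrying them to their matching BP_BugHome.
; Tick traces find nearby bugs and homes, switching a four-state Mode that drives camera timelines and velocity-based FOV.
; A downward sphere trace holds the mesh at an adjustable height above ground, while input applies force and torque.
; Interaction attaches or releases bugs, precision mode toggles a top-down view, and hits drain Health.
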(event Custom|ChangeMode
  (params (Mode :type Integer))
  (bind _output_get (Variables|Default|SetMode Mode))
  (if (not (Variables|Default|GetIsPrecisionMode))
    (Variables|/Script/Engine.SpringArmComponent|SetTargetArmLength (Variables|Default|GetSpringArm1) 1e+05))
  (switch int _output_get
    (:0
      (Utilities|FlowControl|Sequence :!label _label
        (:then_0
          (bind _newtrack_1 (Timeline|Timeline_0 Stop)
            (:Update
              (CallFunction|SetFieldOfView _newtrack_1 7e+01)
              (CallFunction|SetCameraArmTarget _newtrack_1 0.0)
              (if (Utilities|IsValid (Variables|Default|GetBugRef))
                _))))
        (:then_1
          (bind _newtrack_1_2 (Timeline|Timeline_1 PlayFromStart)
            (:Update
              (CallFunction|SetCameraArmTarget _newtrack_1_2 0.0)
              (CallFunction|SetFieldOfView _newtrack_1_2 9e+01)
              (Transformation|SetRelativeRotation (Variables|Default|GetSpringArm) (Math|Rotator|MakeRotator 0.0 -2e+01 0.0) false false)
              (Variables|Default|SetIsPrecisionMode false))))))
    (:1
      (Utilities|FlowControl|Sequence :!label _label_2
        (:then_0
          (Timeline|Timeline_1 Stop))
        (:then_1
          (Timeline|Timeline_0 PlayFromStart))))
    (:2
      (goto _label))
    (:3
      (goto _label_2))))

(event EventBeginPlay
  (bind _returnvalue (UserInterface|CreateWidget "/Game/UI/BP_PLayerUI.BP_PLayerUI_C"))
  (Variables|Default|SetUI_PLayer _returnvalue)
  (UserInterface|Viewport|AddtoViewport _returnvalue 0))

(event Collision|EventHit
  (params (MyComp :type Primitive%20Component%20Object%20Reference) (Other :type Actor%20Object%20Reference) (OtherComp :type Primitive%20Component%20Object%20Reference) (bSelfMoved :type Boolean) (HitLocation :type Vector :default "0, 0, 0") (HitNormal :type Vector :default "0, 0, 0") (NormalImpulse :type Vector :default "0, 0, 0") (Hit :type Hit%20Result%20Structure%20%28by%20ref%29))
  (Variables|Default|SetHealth (- (Variables|Default|GetHealth) 0.1)))

(event EventTick
  (params (DeltaSeconds :type Float%20%28single-precision%29))
  (bind _ignoredactors (Variables|Default|GetIgnoredActors))
  (bind _playermesh (Variables|Default|GetPlayerMesh))
  (bind _playermesh_2 (Variables|Default|GetPlayerMesh))
  (bind _playermesh_3 (Variables|Default|GetPlayerMesh))
  (bind _playermesh_4 (Variables|Default|GetPlayerMesh))
  (bind _returnvalue (Transformation|GetWorldLocation _playermesh))
  (bind _returnvalue_2 (Transformation|GetWorldLocation _playermesh_3))
  (bind _returnvalue_3 (Transformation|GetWorldLocation _playermesh_2))
  (bind _relativelocation (Variables|/Script/Engine.SceneComponent|GetRelativeLocation _playermesh_4))
  (bind _returnvalue_4 (- _returnvalue_2 (Math|Vector|MakeVector 1e+03 0.0 5e+04)))
  (bind _returnvalue_5 (+ _returnvalue_3 "0, 0,-200.000000"))
  (bind _returnvalue_6 (+ _relativelocation "0, 0, 0"))
  (Variables|Default|SetDelta%20Seconds DeltaSeconds)
  (Utilities|FlowControl|Sequence
    (:then_0
      (bind _returnvalue_7 (CallFunction|BugNotCatched))
      (if _returnvalue_7
        (CallFunction|LookforBugsAround)))
    (:then_1
      (bind _ismode (CallFunction|IsMode 1))
      (if _ismode
        (bind _outhit (Collision|LineTraceByChannel _returnvalue (- _returnvalue "0, 0,2000.000000") "TraceTypeQuery1" false 0 "None"))
        (bind _asbp_bug (Utilities|Casting|CastToBP_bug (.HitActor (Collision|BreakHitResult _outhit)))
          (:then
            _)
          (:CastFailed
            _))
        (Variables|Default|SetBugRefReady _asbp_bug)))
    (:then_3
      (if false
        (bind _outhit_2 (Collision|LineTraceByChannel _returnvalue_2 _returnvalue_4 "TraceTypeQuery3" false _ignoredactors "None"))
        (else
          (bind _outhit_3 (Collision|SphereTraceByChannel _returnvalue_2 _returnvalue_4 5e+01 "TraceTypeQuery3" false _ignoredactors "None"))))
      (if (Variables|Default|GetKeepDistanceFromTheGround)
        (Variables|Default|SetLandscapeHitAt (.z (.Location (Collision|BreakHitResult _outhit_3))))
        (Transformation|SetRelativeLocation _playermesh_4 (Math|Vector|MakeVector (.x (Math|Interpolation|VInterpTo _relativelocation (Math|Vector|MakeVector (.x _returnvalue_6) (.y _returnvalue_6) (+ (.z (.Location (Collision|BreakHitResult _outhit_3))) (Math|Float|Clamp(Float) (Variables|Default|GetFlyHeight) 1.5e+02 2e+05))) (Variables|Default|GetDelta%20Seconds) 1e+01)) (.y (Math|Interpolation|VInterpTo _relativelocation (Math|Vector|MakeVector (.x _returnvalue_6) (.y _returnvalue_6) (+ (.z (.Location (Collision|BreakHitResult _outhit_3))) (Math|Float|Clamp(Float) (Variables|Default|GetFlyHeight) 1.5e+02 2e+05))) (Variables|Default|GetDelta%20Seconds) 1e+01)) (.z (Math|Interpolation|VInterpTo _relativelocation (Math|Vector|MakeVector (.x _returnvalue_6) (.y _returnvalue_6) (+ (.z (.Location (Collision|BreakHitResult _outhit_3))) (Math|Float|Clamp(Float) (Variables|Default|GetFlyHeight) 1.5e+02 2e+05))) (Variables|Default|GetDelta%20Seconds) 1e+01))) true true)
        (if (not (Variables|Default|GetIsPrecisionMode))
          (Transformation|SetRelativeRotation (Variables|Default|GetSpringArm) (Math|Rotator|MakeRotator 0.0 (Math|Float|Clamp(Float) (/ (Variables|Default|GetFlyHeight) -5e+02) -7e+01 -1e+01) 0.0) false false))))
    (:then_4
      (bind _ismode_2 (CallFunction|IsMode 3))
      (bind _ismode_3 (CallFunction|IsMode 2))
      (if (or _ismode_2 _ismode_3)
        (bind _outhit_4 (Collision|SphereTraceForObjects _returnvalue_5 _returnvalue_5 4e+02 (Variables|Default|GetBugHomesToFind) false (Variables|Default|GetActors%20to%20Ignore) "None"))
        (bind _asbp_bug_home (Utilities|Casting|CastToBP_BugHome (.HitActor (Collision|BreakHitResult _outhit_4)))
          (:then
            (if (== (Variables|/Game/bugs/blueprints/BP_BugHome.BP_BugHome_C|GetOwnerBugRef _asbp_bug_home) (Variables|Default|GetBugRef))
              (CallFunction|ChangeMode 3)))
          (:CastFailed
            (Utilities|Array|Add (Variables|Default|GetActors%20to%20Ignore) (.HitActor (Collision|BreakHitResult _outhit_4)))
            (CallFunction|ChangeMode 2)))))
    (:then_5
      (switch int (Variables|Default|GetMode)
        (:2
          (bind _outactors (Actor|GetAllActorsOfClass "/Game/bugs/blueprints/BP_BugHome.BP_BugHome_C"))
          (for _array_element _outactors
            (if (== (Variables|Default|GetBugRef) (Variables|/Game/bugs/blueprints/BP_BugHome.BP_BugHome_C|GetOwnerBugRef _array_element))
              _)))))
    (:then_6
      (bind _ismode_4 (CallFunction|IsMode))
      (bind _ismode_5 (CallFunction|IsMode 2))
      (if (or _ismode_4 _ismode_5)
        (Utilities|FlowControl|Sequence
          (:then_0
            ;[1 1 1] FOV value based on velocity
            (bind _newtrack_1 (Timeline|Timeline_3 Stop)
              (:Update
                (CallFunction|SetFieldOfView _newtrack_1 (Math|Float|Clamp(Float) (* (Math|Vector|VectorLength (Transformation|GetComponentVelocity (Variables|Default|GetPlayerMesh))) 0.05) 9e+01 1.3e+02)))))
          (:then_1
            (Timeline|Timeline_3 PlayFromStart)))))))

(event Input|ActionEvents|InputActionInteraction
  (params (Key :type Key%20Structure :default "None"))
  (:Pressed
    (if (Utilities|IsValid (Variables|Default|GetBugRef))
      (Default|DetachPlayer (Variables|Default|GetBugRef))
      (Variables|Default|SetBugRefReady 0)
      (Variables|Default|SetBugRef 0)
      (CallFunction|ChangeMode)
      (elif (Utilities|IsValid (Variables|Default|GetBugRefReady))
        (Variables|Default|SetBugRef (Variables|Default|GetBugRefReady))
        (Variables|Default|SetBugFoundRef 0)
        (Default|AttachtoPlayer (Variables|Default|GetBugRef) self)
        (CallFunction|ChangeMode 2)
        (Default|ShowRescueMode (Variables|Default|GetUI_PLayer) 100)))))

(event Input|ActionEvents|InputActionPrecisionMode
  (params (Key :type Key%20Structure :default "None"))
  (bind _springarm1 (Variables|Default|GetSpringArm1))
  (bind _springarm (Variables|Default|GetSpringArm))
  (bind _relativerotation (Variables|/Script/Engine.SceneComponent|GetRelativeRotation _springarm))
  (:Pressed
    (bind _ismode (CallFunction|IsMode 1))
    (bind _ismode_2 (CallFunction|IsMode 3))
    (if (or _ismode _ismode_2)
      (bind _output_get (Variables|Default|SetIsPrecisionMode (not (Variables|Default|GetIsPrecisionMode))))
      (if _output_get
        (Transformation|SetRelativeRotation _springarm (Math|Rotator|MakeRotator (.roll _relativerotation) -89.900002 (.yaw _relativerotation)) false false)
        (Variables|/Script/Engine.SpringArmComponent|SetTargetArmLength _springarm1 -3e+02)
        (Variables|/Script/Engine.SceneCaptureComponent2D|SetFOVAngle (Variables|Default|GetSceneCaptureComponent2D) 35.0)
        (else
          (Transformation|SetRelativeRotation (Variables|Default|GetSpringArm) (Math|Rotator|MakeRotator 0.0 -2e+01 0.0) false false)
          (Variables|/Script/Engine.SpringArmComponent|SetTargetArmLength _springarm1 1e+05))))))

(event Input|AxisEvents|InputAxisStrafe
  (params (AxisValue :type Float%20%28single-precision%29))
  (bind _playermesh (Variables|Default|GetPlayerMesh))
  (Physics|AddForce _playermesh (* (* (* (Math|Vector|GetRightVector _playermesh) 2e+03) AxisValue) (Physics|GetMass (Variables|Default|GetPlayerMesh))) "None" false))

(event Input|AxisEvents|InputAxisMoveUpDown
  (params (AxisValue :type Float%20%28single-precision%29))
  (Variables|Default|SetFlyHeight (Math|Float|Clamp(Float) (+ (* AxisValue 5e+01) (Variables|Default|GetFlyHeight)) 0.0 5e+05)))

(event Input|AxisEvents|InputAxisMoveLR
  (params (AxisValue :type Float%20%28single-precision%29))
  (if true
    (CallFunction|HandleInput2 (stale Input|AxisEvents|InputAxisMoveFB AxisValue) AxisValue)
    (else
      (CallFunction|OldHandleInput AxisValue (stale Input|AxisEvents|InputAxisMoveFB AxisValue)))))

(event Input|AxisEvents|InputAxisMoveFB
  (params (AxisValue :type Float%20%28single-precision%29))
  (if true
    (CallFunction|HandleInput2 AxisValue (stale Input|AxisEvents|InputAxisMoveLR AxisValue))
    (else
      (CallFunction|OldHandleInput (stale Input|AxisEvents|InputAxisMoveLR AxisValue) AxisValue))))

(fn ConstructionScript)

(fn SpawnConstrain
  (bind _returnvalue (Game|SpawnActorfromClass "/Script/Engine.PhysicsConstraintActor" (Transformation|GetRelativeTransform (Variables|Default|GetPlayerMesh)) "Undefined" 0 0))
  (Variables|Default|SetLineRef _returnvalue))

(fn OldHandleInput
  (params (LeftRightAxis :type Float%20%28single-precision%29) (TopDownAxis :type Float%20%28single-precision%29))
  (bind _moveforce (Variables|Default|GetMoveForce))
  (Physics|AddImpulse (Variables|Default|GetPlayerMesh) (Math|Vector|MakeVector (Math|Float|Clamp(Float) (* (Variables|Default|GetDelta%20Seconds) (* TopDownAxis _moveforce)) -1e+04 1e+04) (Math|Float|Clamp(Float) (* (Variables|Default|GetDelta%20Seconds) (* LeftRightAxis _moveforce)) -1e+04 1e+04) 0.0) "None" false))

(fn HandleInput2
  (params (A :type Float%20%28single-precision%29) (A2 :type Float%20%28single-precision%29))
  (bind _playermesh (Variables|Default|GetPlayerMesh))
  (bind _returnvalue (Physics|GetMass _playermesh))
  (Class|PrimitiveComponent|AddTorqueinDegrees (Variables|Default|GetPlayerMesh) (* (Math|Vector|MakeVector 0.0 0.0 (* A2 1e+05)) _returnvalue) "None" false)
  (Physics|AddForce (Variables|Default|GetPlayerMesh) (* (* (Math|Vector|GetForwardVector (Variables|Default|GetPlayerMesh)) (Math|Float|Clamp(Float) (* (Variables|Default|GetDelta%20Seconds) (* A (Variables|Default|GetMoveForce))) -3e+04 3e+04)) _returnvalue) "None" false))

(fn SetFieldOfView
  (params (Alpha :type Float%20%28single-precision%29) (Value :type Float%20%28single-precision%29))
  (bind _camera (Variables|Default|GetCamera))
  (Camera|SetFieldOfView _camera (Math|Interpolation|Ease "EaseOut" Alpha (Variables|/Script/Engine.CameraComponent|GetFieldOfView _camera) Value 1.0)))

(fn SetCameraArmTarget
  (params (Alpha :type Float%20%28single-precision%29) (TargetZValue :type Float%20%28single-precision%29))
  (bind _springarm (Variables|Default|GetSpringArm))
  (Variables|/Script/Engine.SpringArmComponent|SetTargetOffset _springarm (Math|Vector|MakeVector (.x (Variables|/Script/Engine.SpringArmComponent|GetTargetOffset _springarm)) (.y (Variables|/Script/Engine.SpringArmComponent|GetTargetOffset _springarm)) (Math|Interpolation|Ease "EaseOut" Alpha (.z (Variables|/Script/Engine.SpringArmComponent|GetTargetOffset _springarm)) TargetZValue 5.0))))

(fn BugNotCatched
  (return (not (Utilities|IsValid (Variables|Default|GetBugRef)))))

(fn BugCatched
  (return false))

(fn IsMode
  (params (Mode :type Integer))
  (return (== Mode (Variables|Default|GetMode))))

(fn LookforBugsAround
  (bind _playermesh (Variables|Default|GetPlayerMesh))
  (bind _returnvalue (Transformation|GetWorldLocation _playermesh))
  (bind _outhit (Collision|SphereTraceForObjects _returnvalue _returnvalue 4e+02 (Variables|Default|GetBugsObjectsToFind) false 0 "None"))
  (bind _asbp_bug (Utilities|Casting|CastToBP_bug (.HitActor (Collision|BreakHitResult _outhit)))
    (:then
      (if (and (not (Variables|/Game/bugs/blueprints/BP_bug.BP_bug_C|GetRescued _asbp_bug)) (not (Variables|/Script/Engine.Actor|GetbHidden _asbp_bug)))
        (Variables|Default|SetBugFoundRef _asbp_bug)
        (CallFunction|ChangeMode 1)))
    (:CastFailed
      (if (Utilities|IsValid (Variables|Default|GetBugFoundRef))
        (Variables|Default|SetBugFoundRef 0)
        (CallFunction|ChangeMode)))))

(fn IsNotMode
  (params (Mode :type Integer))
  (return (!= (Variables|Default|GetMode) Mode)))

(fn ScaleMinimapBasedonVelocity)